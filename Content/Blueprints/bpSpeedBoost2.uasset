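; Speed boost zone that is meant to push overlapping bpPipoFinal2 actors along the zone's forward vector.
; Box begin and end overlap events open and close a Gate fed by Tick.
; While open, it teleport-offsets each overlapping bpPipoFinal2 every frame by delta time and SpeedBoost.
; The offset is also multiplied by zero, so it produces no movement, and debug "Hello" prints remain.
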(event OnComponentBeginOverlap(Box)
  (params (OverlappedComponent :type Primitive%20Component%20Object%20Reference) (OtherActor :type Actor%20Object%20Reference) (OtherComp :type Primitive%20Component%20Object%20Reference) (OtherBodyIndex :type Integer) (bFromSweep :type Boolean) (SweepResult :type Hit%20Result%20Structure%20%28by%20ref%29))
  (Development|PrintString "Hello")
  (Utilities|Casting|CastTobpPipoFinal2 OtherActor)
  (Development|PrintString "Hello")
  (Utilities|FlowControl|Gate true) ; enters at Open
)

(event OnComponentEndOverlap(Box)
  (params (OverlappedComponent :type Primitive%20Component%20Object%20Reference) (OtherActor :type Actor%20Object%20Reference) (OtherComp :type Primitive%20Component%20Object%20Reference) (OtherBodyIndex :type Integer))
  (Utilities|Casting|CastTobpPipoFinal2 OtherActor)
  (Utilities|FlowControl|Gate true) ; enters at Close
)

(event EventBeginPlay)

(event Collision|EventActorBeginOverlap
  (params (OtherActor :type Actor%20Object%20Reference)))

(event EventTick
  (params (DeltaSeconds :type Float%20%28single-precision%29))
  (Utilities|FlowControl|Gate true
    (:Exit
      (for _array_element (Collision|GetOverlappingActors (Variables|Default|GetBox) "/Game/Blueprints/bpPipoFinal2.bpPipoFinal2_C" :!class /Script/Engine.PrimitiveComponent)
        (Transformation|AddActorWorldOffset _array_element (* (Math|Vector|GetForwardVector (Transformation|GetActorRotation)) (* DeltaSeconds (Variables|Default|GetSpeedBoost) 0.0)) false true)
        (Development|PrintString "Hello")))))

(fn ConstructionScript)