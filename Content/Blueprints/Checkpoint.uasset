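; Checkpoint actor that reports when a bpPipoFinal2 actor passes through it in the forward direction.
; When the actor leaves the Trigger, a dot product of its velocity and the Trigger's forward vector rejects backward or sideways exits.
; A valid exit fires the CheckpointCleared dispatcher with the checkpoint's number, then hides the Trigger and disables its overlap events, so it clears only once.
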(event OnComponentEndOverlap(Trigger)
  (params (OverlappedComponent :type Primitive%20Component%20Object%20Reference) (OtherActor :type Actor%20Object%20Reference) (OtherComp :type Primitive%20Component%20Object%20Reference) (OtherBodyIndex :type Integer))
  (bind _trigger (Variables|Default|GetTrigger))
  (bind _asbp_pipo_final_2 (Utilities|Casting|CastTobpPipoFinal2 OtherActor))
  (if (> (Math|Vector|DotProduct (Transformation|GetVelocity _asbp_pipo_final_2) (Math|Rotator|GetRotationXVector (Transformation|GetWorldRotation (Variables|Default|GetTrigger)))) 0.0)
    (Default|CallCheckpointCleared (Variables|Default|GetCheckpointNumber))
    (Development|SetHiddeninGame _trigger true false)
    (Variables|/Script/Engine.PrimitiveComponent|SetbGenerateOverlapEvents _trigger false)))

(fn ConstructionScript)