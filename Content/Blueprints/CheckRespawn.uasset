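; CheckRespawn is a checkpoint actor that registers when the player character bpPipoFinal2 passes through it in the correct direction.
; When the character leaves the Trigger, a dot product between its velocity and the Arrow's forward vector confirms the direction.
; A valid pass fires CheckPointCleared with the checkpoint's number, then hides the trigger and disables its overlap events, making it single-use.
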(event OnComponentEndOverlap(Trigger)
  (params (OverlappedComponent :type Primitive%20Component%20Object%20Reference) (OtherActor :type Actor%20Object%20Reference) (OtherComp :type Primitive%20Component%20Object%20Reference) (OtherBodyIndex :type Integer))
  (bind _trigger (Variables|Default|GetTrigger))
  ;[1 1 1] Sistema CheckPoint, Clear al pasar por el
  (bind _asbp_pipo_final_2 (Utilities|Casting|CastTobpPipoFinal2 OtherActor))
  (if (> (Math|Vector|DotProduct (Transformation|GetVelocity _asbp_pipo_final_2) (Math|Rotator|GetRotationXVector (Transformation|GetWorldRotation (Variables|Default|GetArrow)))) 0.0)
    (Default|CallCheckPointCleared (Variables|Default|GetCheckPointNumber))
    (Development|SetHiddeninGame _trigger true false)
    (Variables|/Script/Engine.PrimitiveComponent|SetbGenerateOverlapEvents _trigger false)))

(fn ConstructionScript)