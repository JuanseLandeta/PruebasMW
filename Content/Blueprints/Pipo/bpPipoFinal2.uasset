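; Player-driven MiniWheels vehicle (Pipo) with steering and throttle input, boost pads, a gum hazard and homing missiles.
; Tick drives a trace-based air check that clamps rotation, fan playback, a debug speed readout and a delayed stuck/flipped check that destroys the car, prompting the controller to respawn it.
; Overlaps with bpBoostSpeed and bpGum override physics velocity to boost or stop the car.
; Missile launch box-traces ahead for a homing target before spawning BpMisil.
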(event OnComponentEndOverlap(Mesh)
  (params (OverlappedComponent :type Primitive%20Component%20Object%20Reference) (OtherActor :type Actor%20Object%20Reference) (OtherComp :type Primitive%20Component%20Object%20Reference) (OtherBodyIndex :type Integer))
  ;[1 1 1] Ends Boost Speed
  (bind _asbp_boost_speed (Utilities|Casting|CastTobpBoostSpeed OtherActor))
  (Utilities|FlowControl|Delay 1.0)
  (Development|PrintString "Hello")
  (Utilities|FlowControl|Gate true) ; enters at Close
)

(event OnComponentBeginOverlap(Mesh)
  (params (OverlappedComponent :type Primitive%20Component%20Object%20Reference) (OtherActor :type Actor%20Object%20Reference) (OtherComp :type Primitive%20Component%20Object%20Reference) (OtherBodyIndex :type Integer) (bFromSweep :type Boolean) (SweepResult :type Hit%20Result%20Structure%20%28by%20ref%29))
  (bind _vehiclemovement (Variables|Default|GetVehicleMovement))
  (bind _updatedprimitive (Variables|/Script/Engine.MovementComponent|GetUpdatedPrimitive _vehiclemovement))
  ;[1 1 1] Executes bpBoostSpeed
  (Utilities|Casting|CastTobpBoostSpeed OtherActor)
  (Utilities|FlowControl|Sequence
    (:then_0
      (bind _returnvalue (Physics|GetPhysicsLinearVelocity _updatedprimitive "None"))
      (Utilities|FlowControl|Sequence
        (:then_0
          (Physics|SetPhysicsLinearVelocity _updatedprimitive (* (Math|Vector|ClampVectorSize _returnvalue 2e+03 2e+03) (Variables|Floats|GetBoostSpeed)) false "None"))
        (:then_1
          (Variables|Default|SetBoostExitSpeed (* (Math|Vector|ClampVectorSize _returnvalue 2e+03 2e+03) (Variables|Floats|GetBoostSpeed))))))
    (:then_1
      ;[1 1 1] Ends Boost Speed
      (Utilities|FlowControl|Gate true
        (:Exit
          (for _array_element 0
            (Transformation|AddActorWorldOffset _array_element (* (Math|Vector|GetForwardVector (Transformation|GetActorRotation)) (* (stale EventTick DeltaSeconds) (Variables|Floats|GetBoostSpeed))) false true)))))))

(event Custom|InitAirCheck
  ;[1 1 1] Are we in the air?-if true block rotations
  (Timeline|AirTraceTimeline Play
    (:Update
      (bind _inair_ (CallFunction|AirCheck (Variables|Floats|GetAirTraceDistance) (Variables|Default|GetTracePoint)))
      (if _inair_
        (CallFunction|AirBlock)
        (Development|PrintString "Air Correct Active")))))

(event Custom|InitIsInMotion/RespawnCheck
  ;[1 1 1] Are we stuck?, if true, destroy actor and respawn at last CP
  (bind _stuck_ (CallFunction|IsinMotion/RespawnCheck))
  (if _stuck_
    (bind _stuck__2 (CallFunction|IsinMotion/RespawnCheck))
    (if _stuck__2
      (Development|PrintString "stuck")
      (Utilities|FlowControl|Delay 5.0)
      (Actor|DestroyActor))
    (else
      (Development|PrintString "In Motion"))))

(event EventBeginPlay
  ;[1 1 1] Get initial position for respawn if needed before clearing 1st CheckPoint
  (bind _asmini_wheels_player_cont (Utilities|Casting|CastToMiniWheelsPlayerCont (Game|GetPlayerController 0)))
  (bind _output_get (Variables|Default|SetControllerReference _asmini_wheels_player_cont))
  (Variables|/Game/Blueprints/MiniWheelsPlayerCont.MiniWheelsPlayerCont_C|SetRespawnLocation _output_get (Transformation|GetActorTransform))
  (Utilities|FlowControl|Sequence
    (:then_0
      (CallFunction|InitCarAttributes))))

(event Collision|EventActorBeginOverlap
  (params (OtherActor :type Actor%20Object%20Reference)))

(event EventDestroyed
  ;[1 1 1] Are we stuck?, if true, destroy actor and respawn at last CP
  (Default|RespawnVehicle (Variables|Default|GetControllerReference)))

(event EventTick
  (params (DeltaSeconds :type Float%20%28single-precision%29))
  ;[1 1 1] Initialices Main Functions for the car
  (Variables|Floats|SetDeltaTime DeltaSeconds)
  (Utilities|FlowControl|Sequence
    (:then_0
      ;[1 1 1] Ends Boost Speed
      (Utilities|FlowControl|Gate true) ; enters at Open
    )
    (:then_1
      (CallFunction|InitAirCheck)
      (CallFunction|FanPlayback)
      (Utilities|FlowControl|Delay 2.0)
      (CallFunction|InitIsinMotion/RespawnCheck)
      (CallFunction|Kms/hDisplay))))

(event Input|AxisEvents|InputAxisRight
  (params (AxisValue :type Float%20%28single-precision%29))
  ;[1 1 1] Input Actions
  (Class|WheeledVehicleMovementComponent|SetSteeringInput (Variables|Default|GetVehicleMovement) AxisValue))

(event Input|AxisEvents|InputAxisForward
  (params (AxisValue :type Float%20%28single-precision%29))
  ;[1 1 1] Input Actions
  (Class|WheeledVehicleMovementComponent|SetThrottleInput (Variables|Default|GetVehicleMovement) AxisValue))

(event OnComponentBeginOverlap(GumPU_Collision)
  (params (OverlappedComponent :type Primitive%20Component%20Object%20Reference) (OtherActor :type Actor%20Object%20Reference) (OtherComp :type Primitive%20Component%20Object%20Reference) (OtherBodyIndex :type Integer) (bFromSweep :type Boolean) (SweepResult :type Hit%20Result%20Structure%20%28by%20ref%29))
  ;[1 1 1] Cast to Gum PU Functionality
  (Utilities|Casting|CastTobpGum OtherActor)
  (CallFunction|GumPUFunction)
  (Utilities|FlowControl|Delay 0.5)
  (Variables|Floats|SetThrotle%20Value 1.0))

(event OnComponentEndOverlap(GumPU_Collision)
  (params (OverlappedComponent :type Primitive%20Component%20Object%20Reference) (OtherActor :type Actor%20Object%20Reference) (OtherComp :type Primitive%20Component%20Object%20Reference) (OtherBodyIndex :type Integer))
  ;[1 1 1] Cast to Gum PU Functionality
)

(event Input|ActionEvents|InputActionMissileLaunch
  (params (Key :type Key%20Structure :default "AnyKey"))
  (:Pressed
    (CallFunction|TargetCheck (Variables|Floats|GetMissileTraceDistance) (Variables|Character|GetMesh))
    (bind _returnvalue (Game|SpawnActorfromClass "/Game/PowerUps/bpMisil.bpMisil_C" (Math|Transform|MakeTransform (Transformation|GetWorldLocation (Variables|Default|GetSphere)) (Transformation|GetWorldRotation (Variables|Character|GetMesh))) "Undefined" 0 0))
    (Default|HommingMissile _returnvalue (Variables|Default|GetHomingTarget))))

(fn ConstructionScript)

(fn AirCheck
  (params (TraceDistance :type Float%20%28single-precision%29) (TracePoint :type Scene%20Component%20Object%20Reference))
  (bind _returnvalue (Transformation|GetWorldLocation TracePoint))
  (bind _returnvalue_2 (Collision|LineTraceByChannel _returnvalue (+ _returnvalue (Math|Vector|MakeVector 0.0 0.0 TraceDistance)) "TraceTypeQuery1" false 0 "None"))
  (if _returnvalue_2
    (Variables|Booleans|SetIsInAir? false)
    (Variables|Booleans|SetAllowRotBlock false)
    (else
      (Variables|Booleans|SetIsInAir? true)
      (Variables|Booleans|SetAllowRotBlock true)))
  (return (Variables|Booleans|GetIsInAir?)))

(fn AirBlock
  (bind _mesh (Variables|Character|GetMesh))
  (bind _returnvalue (Transformation|GetWorldRotation _mesh))
  (bind (_roll _pitch _yaw) (Math|Rotator|BreakRotator _returnvalue))
  ;[1 1 1] Bloquea Rotacion en Aire
  (Transformation|SetActorRotation (Math|Rotator|Lerp(Rotator) (Math|Rotator|MakeRotator _roll _pitch _yaw) (Math|Rotator|MakeRotator (Math|Float|ClampAngle _roll -1e+01 1e+01) (Math|Float|ClampAngle _pitch 0.0 1.8e+02) (Math|Float|ClampAngle _yaw -135.0 135.0)) 1.5) true)
  (return))

(fn InitCarAttributes
  (CallFunction|InitAirCheck)
  (return))

(fn IsinMotion/RespawnCheck
  (Variables|Booleans|SetIsInAir? false)
  (if (or (< (Class|WheeledVehicleMovementComponent|GetForwardSpeed (Variables|Default|GetVehicleMovement)) 0.1) (< (Math|Vector|DotProduct (Transformation|GetActorUpVector) "0, 0,1.000000") 0.1))
    (bind _output_get (Variables|Booleans|SetStuck? true))
    (else
      (Variables|Booleans|SetStuck? false)))
  (return _output_get))

(fn CharacterLocation
  (params (TracePoint :type Scene%20Component%20Object%20Reference))
  (bind _output_get (Variables|Default|SetCarPosition (Transformation|GetWorldLocation TracePoint)))
  (return _output_get))

(fn FanPlayback
  (Components|Timeline|SetPlayRate (Variables|Default|GetVent) (* (Class|WheeledVehicleMovementComponent|GetForwardSpeed (Variables|Default|GetVehicleMovement)) 0.001))
  (return))

(fn Kms/hDisplay
  (Development|PrintString (Utilities|String|ToString(Float) (* (Class|WheeledVehicleMovementComponent|GetForwardSpeed (Variables|Default|GetVehicleMovement)) 0.036)))
  (return))

(fn GumPUFunction
  (bind _vehiclemovement (Variables|Default|GetVehicleMovement))
  (bind _updatedprimitive (Variables|/Script/Engine.MovementComponent|GetUpdatedPrimitive _vehiclemovement))
  (Variables|Floats|SetThrotle%20Value 0.0)
  (bind _returnvalue (Physics|GetPhysicsLinearVelocity _updatedprimitive "None"))
  (Variables|Default|SetGumInitSpeed _returnvalue)
  (Physics|SetPhysicsLinearVelocity _updatedprimitive "0, 0, 0" false "None"))

(fn TargetCheck
  (params (TraceDistance :type Float%20%28single-precision%29) (TracePoint :type Scene%20Component%20Object%20Reference))
  (bind _carposition (Variables|Default|GetCarPosition))
  (bind (_outhit _returnvalue) (Class|KismetSystemLibrary|BoxTraceSingleforObjects _carposition (+ _carposition (* (Math|Vector|GetForwardVector TracePoint) TraceDistance)) "20.000000,10000.000000,500.000000" "0.000000,0.000000,0.000000" (Variables|Default|GetObjectsToTarget) false 0 "None" true))
  (bind _output_get (LocalVariables|SetHasTarget? _returnvalue))
  (if _output_get
    (Development|PrintString "Target" false false)
    (Variables|Default|SetHomingTarget (.HitComponent (Collision|BreakHitResult _outhit)))
    (else
      (Development|PrintString "No Target" false false)
      (Variables|Default|SetHomingTarget 0)))
  (return (LocalVariables|GetHasTarget?)))