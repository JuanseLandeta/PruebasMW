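; Race tracker that manages checkpoint order, laps and completion for a MiniWheels race.
; On BeginPlay it copies lap count, medal times and default bests to the player controller, starts game setup, then numbers checkpoints and binds their cleared callback.
; Each clear enables the next checkpoint's trigger and moves the respawn point.
; The last checkpoint updates the lap and either loops to the first or flags completion, calling the controller's Restart.
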(event Custom|ApplySettings
  (bind _controllerreference (Variables|Default|GetControllerReference))
  ;[1 1 1] Aplica Settings de Actualizar tiempos y setear el juego
  (Variables|/Game/Blueprints/MiniWheelsPlayerCont.MiniWheelsPlayerCont_C|SetMaxLaps _controllerreference (Variables|CustomSettings|GetMaxLaps))
  (CallFunction|UpdateTimes)
  (Default|StartGameSetup _controllerreference))

(event Custom|StartSequence
  (bind _checkpoints (Variables|Checkpoints|GetCheckpoints))
  ;[1 1 1] Sequencia de Loop por cada CheckPoint
  (for (_array_element _array_index) (Variables|Checkpoints|GetCheckpoints)
    (Variables|/Game/Blueprints/Checkpoint.Checkpoint_C|SetCheckpointNumber _array_element (+ _array_index 1))
    (Variables|Default|SetTotalCheckpoints (Utilities|Array|Length _checkpoints))
    (CallFunction|ActivateCheckpoint (Utilities|Array|Get(acopy) _checkpoints))
    (for _array_element_2 (Variables|Checkpoints|GetCheckpoints)
      (EventDispatchers|AssignCheckpointCleared _array_element_2 (delegate Custom|Checkpoint%20Cleared)))))

(event Custom|Checkpoint%20Cleared
  (params (NextCheckpoint :type Integer))
  (bind _controllerreference (Variables|Default|GetControllerReference))
  ;[1 1 1] Sequencia de Loop por cada CheckPoint
  (CallFunction|LapCheck/RespawnLoc NextCheckpoint)
  (if (Variables|/Game/Blueprints/MiniWheelsPlayerCont.MiniWheelsPlayerCont_C|GetRaceComplete? _controllerreference)
    (Default|Restart _controllerreference)))

(event EventBeginPlay
  ;[1 1 1] Setea Referencia a Player Controller
  (bind _asmini_wheels_player_cont (Utilities|Casting|CastToMiniWheelsPlayerCont (Game|GetPlayerController 0)))
  (Variables|Default|SetControllerReference _asmini_wheels_player_cont)
  (CallFunction|ApplySettings)
  (CallFunction|StartSequence))

(fn ConstructionScript)

(fn UpdateTimes
  (bind _controllerreference (Variables|Default|GetControllerReference))
  (Variables|/Game/Blueprints/MiniWheelsPlayerCont.MiniWheelsPlayerCont_C|SetGoldTime _controllerreference (Variables|CustomSettings|GetGoldTime))
  (Variables|/Game/Blueprints/MiniWheelsPlayerCont.MiniWheelsPlayerCont_C|SetSilverTime _controllerreference (Variables|CustomSettings|GetSilverTime))
  (Variables|/Game/Blueprints/MiniWheelsPlayerCont.MiniWheelsPlayerCont_C|SetBronzeTime _controllerreference (Variables|CustomSettings|GetBronzeTime))
  (Variables|/Game/Blueprints/MiniWheelsPlayerCont.MiniWheelsPlayerCont_C|SetDefaultBestLapTime _controllerreference (Variables|CustomSettings|GetDefaultBestLap))
  (Variables|/Game/Blueprints/MiniWheelsPlayerCont.MiniWheelsPlayerCont_C|SetDefaultBestRaceTime _controllerreference (Variables|CustomSettings|GetDefaultBestTime)))

(fn LapCheck/RespawnLoc
  (params (Checkpoint :type Integer))
  (bind _output_get (LocalVariables|SetLocalCheckpoint Checkpoint))
  (if (== _output_get (Variables|Default|GetTotalCheckpoints))
    (bind _isracecomplete_ (CallFunction|RaceCompleteCheck))
    (if _isracecomplete_
      _
      (else
        (CallFunction|ActivateCheckpoint (Utilities|Array|Get(acopy) (Variables|Checkpoints|GetCheckpoints)))))
    (Default|UpdateLap (Variables|Default|GetControllerReference))
    (else
      (CallFunction|ActivateCheckpoint (Utilities|Array|Get(acopy) (Variables|Checkpoints|GetCheckpoints) (LocalVariables|GetLocalCheckpoint)))))
  (Variables|/Game/Blueprints/MiniWheelsPlayerCont.MiniWheelsPlayerCont_C|SetRespawnLocation (Variables|Default|GetControllerReference) (Transformation|GetActorTransform (Utilities|Array|Get(acopy) (Variables|Checkpoints|GetCheckpoints) (- (LocalVariables|GetLocalCheckpoint) 1)))))

(fn ActivateCheckpoint
  (params (Next%20Checkpoint :type Checkpoint%20Object%20Reference))
  (bind _trigger (Variables|/Game/Blueprints/Checkpoint.Checkpoint_C|GetTrigger Next%20Checkpoint))
  (Development|SetHiddeninGame _trigger false false)
  (Variables|/Script/Engine.PrimitiveComponent|SetbGenerateOverlapEvents _trigger true))

(fn RaceCompleteCheck
  (bind _controllerreference (Variables|Default|GetControllerReference))
  (bind _controllerreference_2 (Variables|Default|GetControllerReference))
  (if (>= (Variables|/Game/Blueprints/MiniWheelsPlayerCont.MiniWheelsPlayerCont_C|GetActualLap _controllerreference_2) (Variables|/Game/Blueprints/MiniWheelsPlayerCont.MiniWheelsPlayerCont_C|GetMaxLaps _controllerreference_2))
    (bind _output_get (Variables|/Game/Blueprints/MiniWheelsPlayerCont.MiniWheelsPlayerCont_C|SetRaceComplete? _controllerreference true))
    (LocalVariables|SetLocalComplete _output_get)
    (else
      (bind _output_get_2 (Variables|/Game/Blueprints/MiniWheelsPlayerCont.MiniWheelsPlayerCont_C|SetRaceComplete? _controllerreference false))
      (LocalVariables|SetLocalComplete _output_get_2)))
  (return (LocalVariables|GetLocalComplete)))