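; AI-driven gnome racing vehicle that hands itself and three sensor arrows to a VehicleAIModuleRacing component.
; Each tick, a trace reads the surface's physical material to cap AI speed on Grass or Track.
; Tick also starts an air-check timeline that clamps rotation when airborne, and a motion check that only prints moving/stuck debug text.
; Overlapping bpBoostSpeed adds clamped, scaled physics velocity; leaving it applies a delayed forward teleport nudge.
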(event OnComponentEndOverlap(Mesh)
  (params (OverlappedComponent :type Primitive%20Component%20Object%20Reference) (OtherActor :type Actor%20Object%20Reference) (OtherComp :type Primitive%20Component%20Object%20Reference) (OtherBodyIndex :type Integer))
  ;[1 1 1] Termina Boost Speed
  (Utilities|Casting|CastTobpBoostSpeed OtherActor)
  (Utilities|FlowControl|Delay 1.0)
  (for _array_element (Utilities|Array|MakeArray (Variables|Default|GetMinion_reference))
    (Transformation|AddActorWorldOffset _array_element (* (Math|Vector|GetForwardVector (Transformation|GetActorRotation)) (* (stale EventTick _output_get) (Variables|Default|GetBoostSpeed))) false true)))

(event OnComponentBeginOverlap(Mesh)
  (params (OverlappedComponent :type Primitive%20Component%20Object%20Reference) (OtherActor :type Actor%20Object%20Reference) (OtherComp :type Primitive%20Component%20Object%20Reference) (OtherBodyIndex :type Integer) (bFromSweep :type Boolean) (SweepResult :type Hit%20Result%20Structure%20%28by%20ref%29))
  (bind _vehiclemovement (Variables|Default|GetVehicleMovement))
  (bind _updatedprimitive (Variables|/Script/Engine.MovementComponent|GetUpdatedPrimitive _vehiclemovement))
  ;[1 1 1] Ejecuta bpBoostSpeed
  (Utilities|Casting|CastTobpBoostSpeed OtherActor)
  (Utilities|FlowControl|Sequence
    (:then_0
      (bind _returnvalue (Physics|GetPhysicsLinearVelocity _updatedprimitive "None"))
      (Utilities|FlowControl|Sequence
        (:then_0
          (Physics|SetPhysicsLinearVelocity _updatedprimitive (* (Math|Vector|ClampVectorSize _returnvalue 2e+03 2e+03) (Variables|Default|GetBoostSpeed)) true "None"))
        (:then_1
          (Variables|Default|SetBoostInitSpeed (* (Math|Vector|ClampVectorSize _returnvalue 2e+03 2e+03) (Variables|Default|GetBoostSpeed))))))))

(event Custom|InitAirCheck
  ;[1 1 1] Estamos en el aire?-si, bloquea rotacion
  (Timeline|Timeline_0 Play
    (:Update
      (CallFunction|AirCheck (Variables|Default|GetAirTraceDistance))
      (if (Variables|Default|GetIsInAir?)
        (CallFunction|AirBlock)))))

(event Custom|InitIsInMotion
  ;[1 1 1] Estamos Atascados?
  (bind _ismoving_ (CallFunction|IsinMotion))
  (if _ismoving_
    (Utilities|FlowControl|Delay 2.0)
    (Development|PrintString "MINIOMIn Motion" true true "(R=0.000000,G=1.000000,B=0.051178,A=1.000000)")
    (else
      (Utilities|FlowControl|Delay 2.0)
      (Development|PrintString "MINIONStuck" true true "(R=1.000000,G=0.000000,B=0.110346,A=1.000000)"))))

(event EventBeginPlay
  (bind _self self)
  (Class|VehicleAIModuleRacing|SetRequiredProperties (Variables|Default|GetVehicleAIModule_Racing) (Variables|Default|GetRight_detector) (Variables|Default|GetCentralSensor) (Variables|Default|GetLeft_detector) _self _self))

(event EventTick
  (params (DeltaSeconds :type Float%20%28single-precision%29))
  ;[1 1 1] Termina Boost Speed
  (bind _output_get (Variables|Default|SetDeltaTime DeltaSeconds))
  (CallFunction|MatPhysics (Variables|Default|GetMatTraceDistance) (Variables|Default|GetTracePointMinion))
  (CallFunction|InitCarAttributes))

(fn ConstructionScript)

(fn AirCheck
  (params (TraceDistance :type Float%20%28single-precision%29))
  (bind _tracepointminion (Variables|Default|GetTracePointMinion))
  (bind _returnvalue (Transformation|GetWorldLocation _tracepointminion))
  (bind _returnvalue_2 (Collision|LineTraceByChannel _returnvalue (+ _returnvalue (Math|Vector|MakeVector 0.0 0.0 TraceDistance)) "TraceTypeQuery1" true 0 "None"))
  (if _returnvalue_2
    (Variables|Default|SetIsInAir? false)
    (Variables|Default|SetAllowRotBlock false)
    (else
      (Variables|Default|SetIsInAir? true)
      (Variables|Default|SetAllowRotBlock true)))
  (return))

(fn AirBlock
  (bind _mesh (Variables|Character|GetMesh))
  (bind _returnvalue (Transformation|GetWorldRotation _mesh))
  (bind (_roll _pitch _yaw) (Math|Rotator|BreakRotator _returnvalue))
  ;[1 1 1] Bloquea Rotacion en Aire
  (Transformation|SetActorRotation (Math|Rotator|Lerp(Rotator) (Math|Rotator|MakeRotator _roll _pitch _yaw) (Math|Rotator|MakeRotator (Math|Float|ClampAngle _roll -1e+01 1e+01) (Math|Float|ClampAngle _pitch 0.0 1.8e+02) (Math|Float|ClampAngle _yaw -135.0 135.0)) 1.5) true)
  (return))

(fn InitCarAttributes
  (CallFunction|InitAirCheck)
  (CallFunction|InitIsinMotion)
  (return))

(fn IsinMotion
  (bind _vehiclemovement (Variables|Default|GetVehicleMovement))
  (bind _returnvalue (Class|WheeledVehicleMovementComponent|GetForwardSpeed _vehiclemovement))
  (bind _output_get (Variables|Default|SetIsInAir? false))
  (if (or _output_get (and (> _returnvalue 1.0) (> _returnvalue 0.0)))
    (bind _output_get_2 (Variables|Default|SetIsInMotion? true))
    (else
      (bind _output_get_3 (Variables|Default|SetIsInMotion? false))))
  (return _output_get_2 _output_get_3))

(fn CharacterLocation
  (params (TracePointMinion :type Scene%20Component%20Object%20Reference))
  (bind _output_get (Variables|Default|SetCarPosition (Transformation|GetWorldLocation TracePointMinion)))
  (return _output_get))

(fn MatPhysics
  (params (TraceDistance :type Float%20%28single-precision%29) (TracePoint :type Scene%20Component%20Object%20Reference))
  (bind _returnvalue (Transformation|GetWorldLocation TracePoint))
  (bind _vehicleaimodule_racing (Variables|Default|GetVehicleAIModule_Racing))
  (bind (_outhit _returnvalue_2) (Collision|LineTraceByChannel _returnvalue (+ _returnvalue (Math|Vector|MakeVector 0.0 0.0 TraceDistance)) "TraceTypeQuery1" true 0 "Persistent"))
  (if _returnvalue_2
    (switch Utilities|FlowControl|Switch|SwitchonEPhysicalSurface (Variables|/Script/Engine.PhysicalMaterial|GetSurfaceType (.PhysMat (Collision|BreakHitResult _outhit)))
      (:SurfaceType_Default
        _)
      (:SurfaceType1
        (Variables|/Script/BlueMan_VehicleAI.VehicleAIModule_Racing|SetMaxOverallVehicleSpeed _vehicleaimodule_racing 5e+01))
      (:SurfaceType2
        (Variables|/Script/BlueMan_VehicleAI.VehicleAIModule_Racing|SetMaxOverallVehicleSpeed _vehicleaimodule_racing 1.3e+02))))
  (return))