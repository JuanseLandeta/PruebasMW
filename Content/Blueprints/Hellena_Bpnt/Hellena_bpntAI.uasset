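; AI-driven wheeled vehicle Hellena, which races and reacts to speed boost pads.
; BeginPlay feeds left, center and right detector arrows plus the vehicle itself into VehicleAIModuleRacing.
; Entering a bpBoostSpeed adds current velocity scaled by BoostSpeed to the physics body.
; One second after exit, HellenaActor gets a single forward teleport offset scaled by BoostSpeed and the Tick-cached delta time.
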(event OnComponentEndOverlap(Mesh)
  (params (OverlappedComponent :type Primitive%20Component%20Object%20Reference) (OtherActor :type Actor%20Object%20Reference) (OtherComp :type Primitive%20Component%20Object%20Reference) (OtherBodyIndex :type Integer))
  ;[1 1 1] Termina Boost Speed
  (Utilities|Casting|CastTobpBoostSpeed OtherActor)
  (Utilities|FlowControl|Delay 1.0)
  (for _array_element (Utilities|Array|MakeArray (Variables|Default|GetHellena_actor))
    (Transformation|AddActorWorldOffset _array_element (* (Math|Vector|GetForwardVector (Transformation|GetActorRotation)) (* (stale EventTick _output_get) (Variables|Default|GetBoostSpeed))) false true)))

(event OnComponentBeginOverlap(Mesh)
  (params (OverlappedComponent :type Primitive%20Component%20Object%20Reference) (OtherActor :type Actor%20Object%20Reference) (OtherComp :type Primitive%20Component%20Object%20Reference) (OtherBodyIndex :type Integer) (bFromSweep :type Boolean) (SweepResult :type Hit%20Result%20Structure%20%28by%20ref%29))
  (bind _vehiclemovement (Variables|Default|GetVehicleMovement))
  (bind _updatedprimitive (Variables|/Script/Engine.MovementComponent|GetUpdatedPrimitive _vehiclemovement))
  ;[1 1 1] Ejecuta bpBoostSpeed
  (Utilities|Casting|CastTobpBoostSpeed OtherActor)
  (Utilities|FlowControl|Sequence
    (:then_0
      (bind _returnvalue (Physics|GetPhysicsLinearVelocity _updatedprimitive "None"))
      (Utilities|FlowControl|Sequence
        (:then_0
          (bind _output_get (Variables|Default|SetBoostInitSpeed _returnvalue))
          (Physics|SetPhysicsLinearVelocity _updatedprimitive (* _output_get (Variables|Default|GetBoostSpeed)) true "None"))
        (:then_1
          (Variables|Default|SetBoostExitSpeed (* _output_get (Variables|Default|GetBoostSpeed))))))))

(event EventTick
  (params (DeltaSeconds :type Float%20%28single-precision%29))
  ;[1 1 1] Termina Boost Speed
  (bind _output_get (Variables|Default|SetDeltaTime DeltaSeconds)))

(event EventBeginPlay
  (bind _self self)
  (Class|VehicleAIModuleRacing|SetRequiredProperties (Variables|Default|GetVehicleAIModule_Racing) (Variables|Default|GetRight_Detector) (Variables|Default|GetCenter_Detector) (Variables|Default|GetLEft_Detector) _self _self))

(fn ConstructionScript)