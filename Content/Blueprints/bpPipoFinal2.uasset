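; Vehicle pawn Blueprint that accelerates automatically, leaving the player to steer.
; Tick applies ThrotleValue as constant throttle and the Right axis sets steering, while the Forward axis does nothing.
; Overlapping a bpBoostSpeed actor adds a multiple of the current physics velocity, then restores the saved velocity vector after a short delay.
; Disconnected nodes hold unused throttle changes, apparently for slowing in curves.
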(event EventBeginPlay)

(event Collision|EventActorBeginOverlap
  (params (OtherActor :type Actor%20Object%20Reference)))

(event EventTick
  (params (DeltaSeconds :type Float%20%28single-precision%29))
  ;[1 1 1] Inicia Aceleracion Constante
  (bind _output_get (Variables|Default|SetAcelerationTrue true))
  (if _output_get
    (Class|WheeledVehicleMovementComponent|SetThrottleInput (Variables|Default|GetVehicleMovement) (Variables|Default|GetThrotle%20Value))))

(event Input|AxisEvents|InputAxisForward
  (params (AxisValue :type Float%20%28single-precision%29)))

(event Input|AxisEvents|InputAxisRight
  (params (AxisValue :type Float%20%28single-precision%29))
  ;[1 1 1] Controla Curva
  (Class|WheeledVehicleMovementComponent|SetSteeringInput (Variables|Default|GetVehicleMovement) AxisValue))

(event Input|KeyboardEvents|Left
  (params (Key :type Key%20Structure :default "AnyKey"))
  ;[1 1 1] Baja Velocidad en Curva
)

(event Input|KeyboardEvents|A
  (params (Key :type Key%20Structure :default "AnyKey"))
  ;[1 1 1] Baja Velocidad en Curva
)

(event Input|KeyboardEvents|D
  (params (Key :type Key%20Structure :default "AnyKey"))
  ;[1 1 1] Baja Velocidad en Curva
)

(event Input|KeyboardEvents|Right
  (params (Key :type Key%20Structure :default "AnyKey"))
  ;[1 1 1] Baja Velocidad en Curva
)

(event OnComponentBeginOverlap(Mesh)
  (params (OverlappedComponent :type Primitive%20Component%20Object%20Reference) (OtherActor :type Actor%20Object%20Reference) (OtherComp :type Primitive%20Component%20Object%20Reference) (OtherBodyIndex :type Integer) (bFromSweep :type Boolean) (SweepResult :type Hit%20Result%20Structure%20%28by%20ref%29))
  (bind _vehiclemovement (Variables|Default|GetVehicleMovement))
  (bind _updatedprimitive (Variables|/Script/Engine.MovementComponent|GetUpdatedPrimitive _vehiclemovement))
  ;[1 1 1] Ejecuta bpBoostSpeed
  (Utilities|Casting|CastTobpBoostSpeed OtherActor)
  (bind _returnvalue (Physics|GetPhysicsLinearVelocity _updatedprimitive "None"))
  (bind _output_get (Variables|Default|SetBoostInitSpeed _returnvalue))
  (Physics|SetPhysicsLinearVelocity _updatedprimitive (* _output_get (Variables|Default|GetBoostSpeed)) true "None")
  (Utilities|FlowControl|Delay 2.0)
  (Physics|SetPhysicsLinearVelocity (Variables|/Script/Engine.MovementComponent|GetUpdatedPrimitive (Variables|Default|GetVehicleMovement)) (Variables|Default|GetBoostInitSpeed) false "None"))

(fn ConstructionScript)